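; Level manager that starts, restarts and ends rounds in a zombie game.
; On BeginPlay it caches the player, spawn transform and placed enemy and prop marker transforms, then starts the level.
; Each round respawns the player, scatters random props, clears pickups and randomizes directional light rotation.
; After a short delay, a looping timer spawns zombies at random markers until the GameMode-supplied count runs out.
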(event `self.ReceiveBeginPlay`
  (bind _asgm_main (cast `/Game/Input/GM_Main` (`GameplayStatics.GetGameMode`)))
  (set `self.Game Mode` _asgm_main)
  (bind _outactors (`GameplayStatics.GetAllActorsOfClass` "/Game/Blueprints/Enemys/BP_EnemyLocation.BP_EnemyLocation_C"))
  (for _array_element _outactors
    (`KismetArrayLibrary.Array_AddUnique` (`self.EnemySpawnPoint`) (`self.GetTransform` _array_element)))
  (bind _outactors_2 (`GameplayStatics.GetAllActorsOfClass` "/Game/Blueprints/Props/BP_PropLocation.BP_PropLocation_C"))
  (for _array_element_2 _outactors_2
    (`KismetArrayLibrary.Array_AddUnique` (`self.RandomLocations`) (`self.GetTransform` _array_element_2)))
  (bind _returnvalue (`GameplayStatics.GetActorOfClass` "/Game/Blueprints/Player/BP_Player.BP_Player_C"))
  (set `self.playerRef` _returnvalue)
  (bind _returnvalue_2 (`GameplayStatics.GetActorOfClass` "/Game/Blueprints/Player/BP_Spawn.BP_Spawn_C"))
  (set `self.PlayerPos` (`self.GetTransform` _returnvalue_2))
  (`self.StartLevel`))

(event `StartLevel`
  (`self.SetPlayer`)
  (`/Game/Input/GM_Main.StartLevel` (`self.Game Mode`))
  (`self.SetProps`)
  (set `self.enemiesToSpawn` (`/Game/Input/GM_Main.EnemiesRemaining` (`self.Game Mode`)))
  (`self.RemovePickUps`)
  (bind _light (`self.GetDirectionalLight`))
  (`self.K2_SetActorRotation` _light (`KismetMathLibrary.MakeRotator` 0.0 (`KismetMathLibrary.RandomFloatInRange` 170.0 350.0)) false)
  (`KismetSystemLibrary.Delay` 2.0)
  ; EnemySpawneer
  (`KismetSystemLibrary.K2_SetTimerDelegate` (delegate `EnemySpawneer`) (`KismetMathLibrary.RandomFloatInRange` 0.5 1.0) (> (`self.enemiesToSpawn`) 0) :!label _label))

(event `RestartLevel`
  (`KismetSystemLibrary.K2_ClearTimer` null "EnemySpawneer")
  (bind _outactors (`GameplayStatics.GetAllActorsOfClass` "/Game/Blueprints/Enemys/BP_Zombie.BP_Zombie_C"))
  (for _array_element _outactors
    (`self.K2_DestroyActor` _array_element))
  (`self.SetPlayer`)
  (`/Game/Input/GM_Main.RestartLevel` (`self.Game Mode`))
  (`self.SetProps`)
  (set `self.enemiesToSpawn` (`/Game/Input/GM_Main.EnemiesRemaining` (`self.Game Mode`)))
  (`self.RemovePickUps`)
  (bind _light (`self.GetDirectionalLight`))
  (`self.K2_SetActorRotation` _light (`KismetMathLibrary.MakeRotator` 0.0 (`KismetMathLibrary.RandomFloatInRange` 170.0 350.0)) false)
  (`KismetSystemLibrary.Delay` 2.0)
  (goto _label))

(event `EnemySpawneer`
  ; EnemySpawneer
  (if (> (`self.enemiesToSpawn`) 0)
    (`|SpawnActorFromClass` "/Game/Blueprints/Enemys/BP_Zombie.BP_Zombie_C" (`KismetArrayLibrary.Array_Random` (`self.EnemySpawnPoint`)) "AlwaysSpawn" "MultiplyWithRoot" null null)
    (set `self.enemiesToSpawn` (- (`self.enemiesToSpawn`) 1))
    (else
      (`KismetSystemLibrary.K2_ClearTimer` null "EnemySpawneer"))))

(event `SetProps`
  (bind _savedprops (`self.SavedProps`))
  ; SetUpProps
  (for _array_element _savedprops
    (`self.K2_DestroyActor` _array_element))
  (`KismetArrayLibrary.Array_Clear` _savedprops)
  (for _ (range (+ (`KismetArrayLibrary.Array_Length` (`self.RandomLocations`)) 1))
    (bind _returnvalue (`|SpawnActorFromClass` (`KismetArrayLibrary.Array_Random` (`self.Props`)) (`KismetArrayLibrary.Array_Random` (`self.RandomLocations`)) "AlwaysSpawn" "MultiplyWithRoot" null null))
    (`KismetArrayLibrary.Array_Add` (`self.SavedProps`) _returnvalue)))

(event `RemovePickUps`
  (bind _outactors (`GameplayStatics.GetAllActorsOfClass` "/Game/Blueprints/Points/BP_PickUpPoints.BP_PickUpPoints_C"))
  (for _array_element _outactors
    (`self.K2_DestroyActor` _array_element))
  (bind _outactors_2 (`GameplayStatics.GetAllActorsOfClass` "/Game/Blueprints/Weapons/BP_PickUpWeapon.BP_PickUpWeapon_C"))
  (for _array_element_2 _outactors_2
    (`self.K2_DestroyActor` _array_element_2))
  (bind _outactors_3 (`GameplayStatics.GetAllActorsOfClass` "/Game/Blueprints/Shield/BP_PickUpShield.BP_PickUpShield_C"))
  (for _ _outactors_3
    (`self.K2_DestroyActor`)))

(event `SetPlayer`
  (`/Game/Blueprints/Player/BP_Player.Respawn` (`self.playerRef`) (`self.PlayerPos`)))

(event `GameOver`
  (`KismetSystemLibrary.K2_ClearTimer` null "EnemySpawneer")
  (bind _outactors (`GameplayStatics.GetAllActorsOfClass` "/Game/Blueprints/Enemys/BP_Zombie.BP_Zombie_C"))
  (for _array_element _outactors
    (`self.K2_DestroyActor` _array_element)))

(fn `GetDirectionalLight`
  (returns (Light :type "DirectionalLight Object Reference"))
  (bind _returnvalue (`GameplayStatics.GetActorOfClass` "/Script/Engine.DirectionalLight"))
  (return _returnvalue))

(fn `UserConstructionScript`)