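; Enemy character BP_Zombie, animated as a velociraptor, that chases the player and plays an attack montage at close range.
; BeginPlay picks a random walk speed for movement and the anim blueprint, then starts a self-restarting AIMoveTo; Tick drives range checks and the roar timer.
; Die unpossesses it, disables collision, tweens a dither dissolve, notifies GM_Main, may drop a weapon or shield pickup, then destroys the actor.
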(event `self.ReceiveBeginPlay`
  (`self.SetMovementSpeed`)
  (`self.MoveToPlayer`))

(event `self.ReceiveTick`
  (params (DeltaSeconds :type "Float (single-precision)"))
  (`self.PlayRoar` DeltaSeconds)
  (if (not (`self.isDead`))
    (`self.GetPlayerPosition`)
    (if (<= (`self.GetDistanceTo` self (`self.PlayerRef`)) 250.0)
      (if (not (`self.attacking`))
        (set `self.attacking` true)
        (`|PlayMontage` (`self.Mesh`) "/Game/Animations/Zombie/AM_VelociraptorAttack.AM_VelociraptorAttack"
          (:`then`
            (`GameplayStatics.PlaySound2D` "/Game/SoundCue/Anima_Sfx_Pack/CUE/Tiger/Animal_Tiger_10_Cue.Animal_Tiger_10_Cue" 1.0 1.0 0.0 null null))
          (:`OnCompleted`
            (set `self.attacking` false)))))))

(event `MoveToPlayer`
  (bind _asbp_player (cast `/Game/Blueprints/Player/BP_Player` (`GameplayStatics.GetPlayerCharacter` 0)))
  (bind _output_get (set `self.PlayerRef` _asbp_player))
  (`|AIMoveTo` self (`self.PlayerPosition`) _output_get 0.0
    (:`OnSuccess`
      _)
    (:`OnFail`
      _))
  (`self.MoveToPlayer`))

(event `GetPlayerPosition`
  (set `self.PlayerPosition` (`self.K2_GetActorLocation` (`self.PlayerRef`))))

(event `Die`
  (bind (_returnvalue_location _returnvalue_rotation) (`KismetMathLibrary.BreakTransform` (`self.GetTransform`)))
  (bind _returnvalue (`KismetMathLibrary.RandomIntegerInRange` 0 8))
  (bind _returnvalue_location_2 (`KismetMathLibrary.BreakTransform` (`self.GetTransform`)))
  (bind _returnvalue_2 (`self.GetController`))
  (bind _dithermask (`self.ditherMask`))
  (bind _runtimematerial (`/Game/BP_RuntimeMaterial.runtimeMaterial` (`self.BP_RuntimeMaterial`)))
  (`/Engine/EditorBlueprintResources/StandardMacros.IsValid` _returnvalue_2
    (:`Is Valid`
      (`Controller.UnPossess` _returnvalue_2)
      (`GameplayStatics.PlaySoundAtLocation` "/Game/SoundCue/Anima_Sfx_Pack/SC_ZombieDeath.SC_ZombieDeath" _returnvalue_location_2 (struct) 1.0 1.0 0.0 null null null null)
      (set `CharacterMovementComponent.MaxWalkSpeed` 0.0 (`self.CharacterMovement`))
      (`PrimitiveComponent.SetCollisionEnabled` (`self.CapsuleComponent`) "NoCollision")
      (bind _asabp_velociraptor (cast `/Game/Animations/Zombie/ABP_Velociraptor` (`SkeletalMeshComponent.GetAnimInstance` (`self.Mesh`)))
        (:`then`
          (set `/Game/Animations/Zombie/ABP_Velociraptor.dead` true _asabp_velociraptor))
        (:`CastFailed`
          _))
      (set `self.isDead` true)
      (bind _returnvalue_3 (`MaterialInstanceDynamic.K2_GetScalarParameterValue` _runtimematerial _dithermask))
      (bind (_asynctaskproxy _value) (`FCTweenBPActionFloat.TweenFloat` _returnvalue_3 0.0 1.0 "Linear" 0.0 0.0 2.0)
        (:`ApplyEasing`
          (`MaterialInstanceDynamic.SetScalarParameterValue` _runtimematerial _dithermask _value))
        (:`OnComplete`
          (bind _asgm_main (cast `/Game/Input/GM_Main` (`GameplayStatics.GetGameMode`)))
          (`/Game/Input/GM_Main.RemoveEnemy` _asgm_main)
          (if (> _returnvalue 6)
            (`|SpawnActorFromClass` (`KismetArrayLibrary.Array_Random` (`/Game/Input/GM_Main.AllPickUpWeapons` _asgm_main)) (`KismetMathLibrary.MakeTransform` _returnvalue_location _returnvalue_rotation) "AlwaysSpawn" "MultiplyWithRoot" null null)
            (elif (== _returnvalue 3)
              (`|SpawnActorFromClass` "/Game/Blueprints/Shield/BP_PickUpShield.BP_PickUpShield_C" (`KismetMathLibrary.MakeTransform` _returnvalue_location _returnvalue_rotation) "AlwaysSpawn" "MultiplyWithRoot" null null)))
          (`self.K2_DestroyActor`))))))

(event `PlayRoar`
  (params (Time :type "Float (double-precision)"))
  (bind _output_get (set `self.roarTimer` (+ Time (`self.roarTimer`))))
  (if (`self.isDead`)
    (`AudioComponent.Stop` (`self.Roar`) :!label _label)
    (elif (`self.Attacking`)
      (goto _label)
      (elif (> _output_get 10.0)
        (`AudioComponent.Play` (`self.Roar`) 0.0)
        (set `self.roarTimer` 0.0)
        (else
          (goto _label))))))

(fn `SetMovementSpeed`
  (bind _returnvalue (`KismetMathLibrary.RandomIntegerInRange` 1 3))
  (bind _charactermovement (`self.CharacterMovement`))
  (if (== _returnvalue 1)
    (bind _output_get (set `CharacterMovementComponent.MaxWalkSpeed` 220.0 _charactermovement))
    (elif (== _returnvalue 2)
      (set `CharacterMovementComponent.MaxWalkSpeed` 260.0 _charactermovement)
      (else
        (if (== _returnvalue 3)
          _
          (else
            _))
        (set `CharacterMovementComponent.MaxWalkSpeed` 300.0 _charactermovement))))
  (bind _asabp_velociraptor (cast `/Game/Animations/Zombie/ABP_Velociraptor` (`SkeletalMeshComponent.GetAnimInstance` (`self.Mesh`))))
  (set `/Game/Animations/Zombie/ABP_Velociraptor.MoveSpeed` _output_get _asabp_velociraptor))

(fn `UserConstructionScript`)