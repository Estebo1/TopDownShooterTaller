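; BP_Exit is a level exit trigger that moves the player on to the next level once the current one is finished.
; When BP_Player overlaps its Box, it checks that GM_Main reports the level finished but not the game.
; It then clears the finished flag through BP_LevelManager's GameMode reference, triggers the next-level fade-out and starts the level after a short delay.
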(event `self.ReceiveBeginPlay`
  (bind _asgm_main (cast `/Game/Input/GM_Main` (`GameplayStatics.GetGameMode`)))
  (set `self.GameMode` _asgm_main))

(event `self.Box.OnComponentBeginOverlap`
  (params (OverlappedComponent :type "PrimitiveComponent Object Reference") (OtherActor :type "Actor Object Reference") (OtherComp :type "PrimitiveComponent Object Reference") (OtherBodyIndex :type Integer) (bFromSweep :type Boolean) (SweepResult :type "HitResult Structure (by ref)"))
  (bind _gamemode (`self.GameMode`))
  (if (`GameplayStatics.ObjectIsA` OtherActor "/Game/Blueprints/Player/BP_Player.BP_Player_C")
    (if (`/Game/Input/GM_Main.finishedLevel` _gamemode)
      (if (not (`/Game/Input/GM_Main.finishedGame` _gamemode))
        (bind _returnvalue (`GameplayStatics.GetActorOfClass` "/Game/Blueprints/BP_LevelManager.BP_LevelManager_C"))
        (bind _game_mode (`/Game/Blueprints/BP_LevelManager.Game Mode` _returnvalue))
        (set `/Game/Input/GM_Main.finishedLevel` false _game_mode)
        (`/Game/Input/GM_Main.UseFadeOutNextLevel` _game_mode)
        (`KismetSystemLibrary.Delay` 3.0)
        (`/Game/Input/GM_Main.StartLevel` _game_mode)))))

(fn `UserConstructionScript`)