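; Player character for a cursor-aimed shooter with a limited number of lives.
; Enhanced Input drives camera-yaw-relative movement and montage-backed firing through the weapon component, while Tick smoothly yaws the body toward the cursor hit point.
; LoseLife sets the AnimBP death flag, plays a sound, then has GM_Main end the game or fade and restart the level.
; Respawn repositions and revives the player; debug key U forces a death.
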(event Custom|LoseLife
  (bind _gamemodereference (Variables|Default|GetGameModeReference))
  (Variables|Default|SetLifes (- (Variables|Default|GetLifes) 1))
  (Variables|/Game/Animations/Player/ABP_Player.ABP_Player_C|Setdead (Variables|Default|GetabpPlayer) true)
  (Variables|Default|SetisDead true)
  (Audio|Components|Audio|Play (Variables|Default|GetDyingSound) 0.0)
  (Utilities|FlowControl|Delay 1.0)
  (if (<= (Variables|Default|GetLifes) 0)
    (Default|Lose _gamemodereference)
    (else
      (Default|LoseLife _gamemodereference)
      (Default|UseFadeOutRestartLevel _gamemodereference)
      (Utilities|FlowControl|Delay 2.0)
      (Default|RestartLevel _gamemodereference))))

(event Custom|Respawn
  (params (Location :type Transform))
  (if (Utilities|IsValid (Variables|Default|GetabpPlayer))
    _
    (else
      (CallFunction|GetAnimationBp)))
  (Transformation|SetActorTransform Location)
  (Variables|/Game/Animations/Player/ABP_Player.ABP_Player_C|Setdead (Variables|Default|GetabpPlayer) false)
  (Variables|Default|SetisDead false)
  (Audio|Components|Audio|Stop (Variables|Default|GetDyingSound)))

(event Input|EnhancedActionEvents|EnhancedInputActionIA_Move
  (params (ActionValue :type Vector%202D%20Structure) (ElapsedSeconds :type Float%20%28double-precision%29) (TriggeredSeconds :type Float%20%28double-precision%29) (InputAction :type Input%20Action%20Object%20Reference :default "/Game/Input/IA_Move.IA_Move"))
  ;[0.15 0.15 0.15 0.5] Movement
  (if (not (Variables|Default|GetisDead))
    (CallFunction|Move (.x ActionValue) (.y ActionValue))))

(event Input|EnhancedActionEvents|EnhancedInputActionIA_Shoot
  (params (ActionValue :type Boolean) (ElapsedSeconds :type Float%20%28double-precision%29) (TriggeredSeconds :type Float%20%28double-precision%29) (InputAction :type Input%20Action%20Object%20Reference :default "/Game/Input/IA_Shoot.IA_Shoot"))
  ;[0.15 0.15 0.15 0.5] Shoot
  (if (not (Variables|Default|GetisDead))
    (Animation|Montage|PlayMontage (Variables|Character|GetMesh) "/Game/Animations/Player/AM_PlayerShooting.AM_PlayerShooting"
      (:then
        (Default|Shoot (Variables|Default|GetBP_Weapons))))))

(event EventBeginPlay
  (Input|AddMappingContext (PlayerController|LocalPlayerSubsystems|GetEnhancedInputLocalPlayerSubsystem (Game|GetPlayerController 0)) "/Game/Input/IMC_Player.IMC_Player" 0 "(bIgnoreAllPressedKeysUntilRelease=True,bForceImmediately=False,bNotifyUserSettings=False)")
  (CallFunction|GetAnimationBp)
  (Variables|Default|SetisDead false)
  (bind _asgm_main (Utilities|Casting|CastToGM_Main (Game|GetGameMode)))
  (Variables|Default|SetGameModeReference _asgm_main))

(event EventTick
  (params (DeltaSeconds :type Float%20%28single-precision%29))
  (bind _self self)
  (bind _returnvalue (Transformation|GetActorTransform _self))
  ;[0.15 0.15 0.15 0.5] LookAt
  (if (not (Variables|Default|GetisDead))
    (Transformation|SetActorRotation (Math|Rotator|MakeRotator 0.0 0.0 (- (.yaw (Math|Interpolation|RInterpTo (.rotation _returnvalue) (Math|Rotator|FindLookatRotation (.location _returnvalue) (.Location (Collision|BreakHitResult (.HitResult (Game|Player|GetHitResultUnderCursorbyChannel (Game|GetPlayerController 0) "TraceTypeQuery1" true))))) DeltaSeconds 3e+01)) 3.0)))))

(event Input|KeyboardEvents|DebugKeyU
  (params (Key :type Key%20Structure :default "None") (ActionValue :type Input%20Action%20Value%20Structure))
  (:Pressed
    (CallFunction|LoseLife)))

(fn ConstructionScript)

(fn Move
  (params (X%20Value :type Float%20%28double-precision%29) (Y%20Value :type Float%20%28double-precision%29))
  (bind _returnvalue (Pawn|GetControlRotation :!class /Script/Engine.Pawn))
  (Pawn|Input|AddMovementInput (Math|Vector|GetRightVector (Math|Rotator|MakeRotator (.roll _returnvalue) 0.0 (.yaw _returnvalue))) X%20Value false)
  (Pawn|Input|AddMovementInput (Math|Vector|GetForwardVector (Math|Rotator|MakeRotator 0.0 0.0 (.yaw (Pawn|GetControlRotation :!class /Script/Engine.Pawn)))) Y%20Value false))

(fn Shoot
  (Game|SpawnActorfromClass "/Game/Blueprints/Weapons/Launcher/Bullet.Bullet_C" (Transformation|GetWorldTransform (Variables|Default|GetBulletPoint)) "Undefined" "MultiplyWithRoot" 0 0))

(fn GetAnimationBp
  (bind _asabp_player (Utilities|Casting|CastToABP_Player (Components|SkeletalMesh|GetAnimInstance (Variables|Character|GetMesh))))
  (Variables|Default|SetabpPlayer _asabp_player))

(fn UpdateAnimBlueprint
  (bind _abpplayer (Variables|Default|GetabpPlayer)
    (:then
      (Variables|/Game/Animations/Player/ABP_Player.ABP_Player_C|SetMoveSpeed _abpplayer (Variables|Default|GetcurrentMovement)))
    (:else)))