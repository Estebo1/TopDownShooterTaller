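; BP_Fire is a flamethrower weapon Blueprint that kills zombies touched by its fire.
; StartFire enables collision on the Fire component and spawns a one-shot P_Flamethrower emitter at ShootingPoint, with a direction built from that point's rotation components.
; StopFire and BeginPlay disable the collision, without touching the emitter.
; Any BP_Zombie that begins overlapping Fire has Die called on it immediately.
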(event `self.ReceiveBeginPlay`
  (`parent.ReceiveBeginPlay`)
  (`PrimitiveComponent.SetCollisionEnabled` (`self.Fire`) "NoCollision"))

(event `/Game/Blueprints/Weapons/IFire.StartFire`
  (bind _shootingpoint (`self.ShootingPoint`))
  (bind (_returnvalue_roll _returnvalue_pitch _returnvalue_yaw) (`KismetMathLibrary.BreakRotator` (`SceneComponent.K2_GetComponentRotation` _shootingpoint)))
  (`PrimitiveComponent.SetCollisionEnabled` (`self.Fire`) "QueryAndPhysics")
  (`GameplayStatics.SpawnEmitterAtLocation` "/Game/Realistic_Starter_VFX_Pack_Vol2/Particles/Fire/P_flamethrower.P_Flamethrower" (`SceneComponent.K2_GetComponentLocation` _shootingpoint) (`KismetMathLibrary.Conv_VectorToRotator` (`KismetMathLibrary.MakeVector` _returnvalue_roll (- _returnvalue_pitch 45.0) _returnvalue_yaw))))

(event `/Game/Blueprints/Weapons/IFire.StopFire`
  (`PrimitiveComponent.SetCollisionEnabled` (`self.Fire`) "NoCollision"))

(event `self.Fire.OnComponentBeginOverlap`
  (params (OverlappedComponent :type "PrimitiveComponent Object Reference") (OtherActor :type "Actor Object Reference") (OtherComp :type "PrimitiveComponent Object Reference") (OtherBodyIndex :type Integer) (bFromSweep :type Boolean) (SweepResult :type "HitResult Structure (by ref)"))
  (if (`GameplayStatics.ObjectIsA` OtherActor "/Game/Blueprints/Enemys/BP_Zombie.BP_Zombie_C")
    (bind _asbp_zombie (cast `/Game/Blueprints/Enemys/BP_Zombie` OtherActor))
    (`/Game/Blueprints/Enemys/BP_Zombie.Die` _asbp_zombie)))

(fn `UserConstructionScript`
  (`parent.UserConstructionScript`))