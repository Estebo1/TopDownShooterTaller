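; BP_Launcher is a launcher weapon Blueprint that fires a projectile with a firework launch sound.
; StartFire, gated by CanShoot, plays the sound, spawns the Bullet class at ShootingPoint and starts a looping FireRate timer.
; That timer repeatedly calls ResetFire to re-enable shooting without firing again.
; StopFire only clears CanShoot and leaves any running timer active.
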(event `self.ReceiveBeginPlay`
  (`parent.ReceiveBeginPlay`)
  (set `self.canShoot` true))

(event `ResetFire`
  (set `self.canShoot` true))

(event `/Game/Blueprints/Weapons/IFire.StartFire`
  (if (`self.canShoot`)
    (set `self.canShoot` false)
    (`GameplayStatics.PlaySound2D` "/Game/SoundCue/SFX_Essentials_FREE_SAMPLE/SFX_Essentials_03_FIREWORKS/Cues/FRWKComr_InsJ_Fireworks_Single_Close_03-14-Launch_Cue.FRWKComr_InsJ_Fireworks_Single_Close_03-14-Launch_Cue" 1.0 1.0 0.0 null null)
    (`|SpawnActorFromClass` "/Game/Blueprints/Weapons/Launcher/Bullet.Bullet_C" (`SceneComponent.K2_GetComponentToWorld` (`self.ShootingPoint`)) "Undefined" "MultiplyWithRoot" null null)
    (`KismetSystemLibrary.K2_SetTimerDelegate` (delegate `ResetFire`) (`self.FireRate`) true)))

(event `/Game/Blueprints/Weapons/IFire.StopFire`
  (set `self.canShoot` false))

(fn `UserConstructionScript`
  (`parent.UserConstructionScript`))