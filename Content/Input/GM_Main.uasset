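; Main game mode that runs level progression, enemy counts, score and win/lose state.
; It creates the HUD on BeginPlay and spawns a fresh BP_LevelManager for each level start or restart.
; Enemy counts scale with Level; clearing all enemies shows the return-house prompt and advances the level, winning past level four.
; HUD events forward fades, hearts, weapon and end screens.
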(event `self.ReceiveBeginPlay`
  (bind _returnvalue (`|CreateWidget` "/Game/Blueprints/Widget/WBP_HUD.WBP_HUD_C"))
  (bind _output_get (set `self.HUDReference` _returnvalue))
  (`UserWidget.AddToViewport` _output_get 0)
  (set `PlayerController.bShowMouseCursor` true (`GameplayStatics.GetPlayerController` 0)))

(event `CreateLevelManager`
  (bind _levelmanager (`self.levelManager`))
  (`/Engine/EditorBlueprintResources/StandardMacros.IsValid` _levelmanager
    (:`Is Valid`
      (`self.K2_DestroyActor` _levelmanager))
    (:`Is Not Valid`
      _))
  (bind _returnvalue (`|SpawnActorFromClass` "/Game/Blueprints/BP_LevelManager.BP_LevelManager_C" (`SceneComponent.K2_GetComponentToWorld` (`self.DefaultSceneRoot`)) "AlwaysSpawn" "MultiplyWithRoot" null null))
  (set `self.levelManager` _returnvalue))

(event `StartLevel`
  (`self.CreateLevelManager`)
  (bind _output_get (set `self.EnemiesRemaining` (* (`self.EnemyCount`) (`self.Level`))))
  (`/Game/Blueprints/Widget/WBP_HUD.EnemyAmounUpdate` (`self.HUDReference`) _output_get)
  (set `self.finishedLevel` false)
  (`self.UseFadeIn`)
  (`/Game/Blueprints/BP_LevelManager.StartLevel` (`self.levelManager`))
  (`self.RemoveReturnHouse`))

(event `RestartLevel`
  (set `self.EnemiesRemaining` (* (`self.EnemyCount`) (`self.Level`)))
  (set `self.finishedLevel` false)
  (`self.UseFadeIn`)
  (`KismetSystemLibrary.Delay` 1.0)
  (`self.CreateLevelManager`)
  (`/Game/Blueprints/BP_LevelManager.RestartLevel` (`self.levelManager`))
  (`self.RemoveReturnHouse`)
  (`/Game/Blueprints/Widget/WBP_HUD.EnemyAmounUpdate` (`self.HUDReference`) (`self.EnemyCount`)))

(event `RemoveEnemy`
  (bind _output_get (set `self.EnemiesRemaining` (- (`self.EnemiesRemaining`) 1)))
  (`/Game/Blueprints/Widget/WBP_HUD.EnemyAmounUpdate` (`self.HUDReference`) _output_get)
  (if (<= _output_get 0)
    (set `self.finishedLevel` true)
    (`self.ShowReturnHouse`)
    (bind _output_get_2 (set `self.Level` (+ (`self.Level`) 1)))
    (if (> _output_get_2 4)
      (`self.Win`))))

(event `AddPoints`
  (params (Added :type Integer))
  (set `self.Points` (+ Added (`self.Points`))))

(event `UseFadeIn`
  (bind _hudreference (`self.HUDReference`))
  (`/Engine/EditorBlueprintResources/StandardMacros.IsValid` _hudreference
    (:`Is Valid`
      (`/Game/Blueprints/Widget/WBP_HUD.ToggleFadeIn` _hudreference false))))

(event `UseFadeOutNextLevel`
  (bind _hudreference (`self.HUDReference`))
  (`/Game/Blueprints/Widget/WBP_HUD.ChangeLevel` _hudreference)
  (`/Game/Blueprints/Widget/WBP_HUD.ToggleFadeIn` _hudreference true))

(event `UseFadeOutRestartLevel`
  (`/Game/Blueprints/Widget/WBP_HUD.ToggleFadeIn` (`self.HUDReference`) true))

(event `Lose`
  (`/Game/Blueprints/Widget/WBP_HUD.Lose` (`self.HUDReference`)))

(event `LoseLife`
  (`/Game/Blueprints/Widget/WBP_HUD.LoseHeart` (`self.HUDReference`)))

(event `SetCurrentWeapon`
  (params (CurrentWeapon :type "/Game/Blueprints/Weapons/BP_Weapon Class Reference"))
  (`/Game/Blueprints/Widget/WBP_HUD.SetCurrentWeapon` (`self.HUDReference`) CurrentWeapon))

(event `Win`
  (set `self.finishedGame` true)
  (`/Game/Blueprints/Widget/WBP_HUD.Win` (`self.HUDReference`)))

(event `ShowReturnHouse`
  (`/Game/Blueprints/Widget/WBP_HUD.ShowRemoveHouse` (`self.HUDReference`)))

(event `RemoveReturnHouse`
  (`/Game/Blueprints/Widget/WBP_HUD.RemoveReturnHouse` (`self.HUDReference`)))

(fn `UserConstructionScript`)